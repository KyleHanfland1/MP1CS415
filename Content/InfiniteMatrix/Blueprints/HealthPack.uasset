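; HealthPack is an actor Blueprint for a health pickup, though its pickup logic is not connected to any event.
; Tick destroys the pack once it is over 10000 units from the player pawn along X, in either direction.
; The orphaned branch would heal BP_Player by 50, capped at 100, print a message and destroy the pack, or just destroy it for other actors.
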(event `self.ReceiveActorBeginOverlap`
  (params (OtherActor :type "Actor Object Reference")))

(event `self.ReceiveTick`
  (params (DeltaSeconds :type "Float (single-precision)"))
  (bind _returnvalue_x (`KismetMathLibrary.BreakVector` (`self.K2_GetActorLocation`)))
  (bind _returnvalue_x_2 (`KismetMathLibrary.BreakVector` (`self.K2_GetActorLocation` (`GameplayStatics.GetPlayerPawn` 0))))
  (if (> (`KismetMathLibrary.Abs` (- _returnvalue_x _returnvalue_x_2)) 10000.0)
    (`self.K2_DestroyActor`)))

(fn `UserConstructionScript`)