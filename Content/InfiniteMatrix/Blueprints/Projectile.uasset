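; Projectile actor that awards the player score for hitting enemies and can destroy health packs.
; On overlap it adds points to BP_Player for an Enemy or destroys a HealthPack, then destroys itself whatever it touched, leaving enemies intact.
; Every tick it rewrites the ProjectileMovement initial and max speed as a base value plus a multiple of the player's score.
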(event `self.ReceiveActorBeginOverlap`
  (params (OtherActor :type "Actor Object Reference"))
  (bind _returnvalue (`GameplayStatics.GetObjectClass` OtherActor))
  (if (== "/Game/InfiniteMatrix/Blueprints/Enemy.Enemy_C" _returnvalue)
    (bind _asbp_player (cast `/Game/InfiniteMatrix/Blueprints/BP_Player` (`GameplayStatics.GetPlayerPawn` 0)))
    (set `/Game/InfiniteMatrix/Blueprints/BP_Player.Score` (+ (`/Game/InfiniteMatrix/Blueprints/BP_Player.Score` _asbp_player) 1000.0) _asbp_player)
    (elif (== "/Game/InfiniteMatrix/Blueprints/HealthPack.HealthPack_C" _returnvalue)
      (`self.K2_DestroyActor` OtherActor)))
  (`self.K2_DestroyActor`))

(event `self.ReceiveTick`
  (params (DeltaSeconds :type "Float (single-precision)"))
  (bind _projectilemovement (`self.ProjectileMovement`))
  (bind _asbp_player (cast `/Game/InfiniteMatrix/Blueprints/BP_Player` (`GameplayStatics.GetPlayerPawn` 0)))
  (bind _returnvalue (+ (* (`/Game/InfiniteMatrix/Blueprints/BP_Player.Score` _asbp_player) 2.0) 3000.0))
  (set `ProjectileMovementComponent.InitialSpeed` _returnvalue _projectilemovement)
  (set `ProjectileMovementComponent.MaxSpeed` _returnvalue _projectilemovement))

(fn `UserConstructionScript`)