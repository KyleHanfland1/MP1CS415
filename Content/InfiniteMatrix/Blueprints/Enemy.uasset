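; Enemy actor for InfiniteMatrix that damages the player on overlap and destroys itself.
; A player hit subtracts health and, at zero or below, flags BP_Player dead and shows the restart display.
; Any other overlap also destroys it, awarding score only on a Projectile class check, whose GetClass has no OtherActor input.
; Tick culls it when too far from the player along X.
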(event `self.ReceiveActorBeginOverlap`
  (params (OtherActor :type "Actor Object Reference"))
  (if (== "/Game/InfiniteMatrix/Blueprints/BP_Player.BP_Player_C" (`GameplayStatics.GetObjectClass` OtherActor))
    (bind _asbp_player (cast `/Game/InfiniteMatrix/Blueprints/BP_Player` OtherActor))
    (bind _output_get (set `/Game/InfiniteMatrix/Blueprints/BP_Player.CurrentHealth` (- (`/Game/InfiniteMatrix/Blueprints/BP_Player.CurrentHealth` _asbp_player) 50.0) _asbp_player))
    (`self.K2_DestroyActor`)
    (if (not (> _output_get 0.0))
      (set `/Game/InfiniteMatrix/Blueprints/BP_Player.IsDead` true _asbp_player)
      (`/Game/InfiniteMatrix/Blueprints/BP_Player.DisplayRestart` _asbp_player))
    (else
      (if (== "/Game/InfiniteMatrix/Blueprints/Projectile.Projectile_C" (`GameplayStatics.GetObjectClass` null))
        (bind _asbp_player_2 (cast `/Game/InfiniteMatrix/Blueprints/BP_Player` (`GameplayStatics.GetPlayerPawn` 0)))
        (set `/Game/InfiniteMatrix/Blueprints/BP_Player.Score` (+ (`/Game/InfiniteMatrix/Blueprints/BP_Player.Score` _asbp_player_2) 1000.0) _asbp_player_2))
      (`self.K2_DestroyActor`))))

(event `self.ReceiveTick`
  (params (DeltaSeconds :type "Float (single-precision)"))
  (bind _returnvalue_x (`KismetMathLibrary.BreakVector` (`self.K2_GetActorLocation`)))
  (bind _returnvalue_x_2 (`KismetMathLibrary.BreakVector` (`self.K2_GetActorLocation` (`GameplayStatics.GetPlayerPawn` 0))))
  (if (> (`KismetMathLibrary.Abs` (- _returnvalue_x _returnvalue_x_2)) 10000.0)
    (`self.K2_DestroyActor`)))

(fn `UserConstructionScript`)